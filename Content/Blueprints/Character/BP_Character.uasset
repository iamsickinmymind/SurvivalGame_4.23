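; BP_Character is a character Blueprint that handles melee-style hit feedback and prints a health value when health changes.
; Point damage feeds PlayerHitFX, which plays a random melee hit montage and spawns the first melee emitter at the impact, aligned to the surface normal.
; The construction script adds the character to its SceneCaptureComponent2D show-only list, so that capture can render the character in isolation.
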(event `self.ReceiveBeginPlay`)

(event `self.OnHealthModified`
  (params (DeltaHealth :type "Float (single-precision)"))
  (`KismetSystemLibrary.PrintString` (`KismetStringLibrary.Conv_DoubleToString` (- (`self.Health`) DeltaHealth))))

(event `self.ReceivePointDamage`
  (params (Damage :type "Float (single-precision)") (DamageType :type "DamageType Object Reference") (HitLocation :type "Vector Structure") (HitNormal :type "Vector Structure") (HitComponent :type "PrimitiveComponent Object Reference") (BoneName :type Name) (ShotFromDirection :type "Vector Structure") (InstigatedBy :type "Controller Object Reference") (DamageCauser :type "Actor Object Reference") (HitInfo :type "HitResult Structure (by ref)"))
  (`self.PlayerHitFX` Damage DamageType HitInfo true))

(event `PlayerHitFX`
  (params (Damage :type "Float (double-precision)") (`Damage Type` :type "DamageType Object Reference") (HitResult :type "HitResult Structure") (`PointDamage?` :type Boolean))
  (bind (_bblockinghit _binitialoverlap _time _distance _location _impactpoint _normal) (`GameplayStatics.BreakHitResult` HitResult))
  (bind _hitfx_animations_melee (`self.HitFX_Animations_Melee`))
  (`self.PlayAnimMontage` (`|GetArrayItem` _hitfx_animations_melee (`KismetMathLibrary.RandomIntegerInRange` 0 (- (`KismetArrayLibrary.Array_Length` _hitfx_animations_melee) 1))))
  (if `PointDamage?`
    (`GameplayStatics.SpawnEmitterAtLocation` (`|GetArrayItem` (`self.HitFX_Emitters_Melee`)) _location (`KismetMathLibrary.Conv_VectorToRotator` _normal))))

(fn `UserConstructionScript`
  (`KismetArrayLibrary.Array_AddUnique` (`SceneCaptureComponent.ShowOnlyActors` (`self.SceneCaptureComponent2D`)) self))