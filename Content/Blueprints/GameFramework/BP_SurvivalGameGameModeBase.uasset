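; Survival game mode Blueprint that assigns each spawning player a random, unused BP_PlayerStart.
; BeginPlay caches every BP_PlayerStart actor in the level into the PlayerStarts array.
; The FindPlayerStart function re-rolls random entries until one is free, marks it used, returns it and prints debug names.
; The retry loop has no exit when every start is already used.
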(event `self.ReceiveBeginPlay`
  (bind _outactors (`GameplayStatics.GetAllActorsOfClass` "/Game/Blueprints/GameFramework/BP_PlayerStart.BP_PlayerStart_C"))
  (set `self.PlayerStarts` _outactors))

(fn `FindPlayerStart`
  (params (Player :type "Controller Object Reference") (IncomingName :type String))
  (returns (ReturnValue :type "Actor Object Reference"))
  (locals (FavouritePlayerStart :type "/Game/Blueprints/GameFramework/BP_PlayerStart Object Reference"))
  (bind _favouriteplayerstart (`local.FavouritePlayerStart`))
  (bind _playerstarts (`self.PlayerStarts`))
  (bind _output (`|GetArrayItem` _playerstarts (`KismetMathLibrary.RandomIntegerInRange` 0 (- (`KismetArrayLibrary.Array_Length` _playerstarts) 1))))
  (set `local.FavouritePlayerStart` _output)
  (while (`/Game/Blueprints/GameFramework/BP_PlayerStart.IsUsed` (`local.FavouritePlayerStart`))
    (bind _output_get (set `local.FavouritePlayerStart` _output))
    (`KismetSystemLibrary.PrintString` (`KismetSystemLibrary.GetDisplayName` _output_get)))
  (`/Game/Blueprints/GameFramework/BP_PlayerStart.MarkUsed` (`local.FavouritePlayerStart`))
  (`KismetSystemLibrary.PrintString` (`KismetSystemLibrary.GetDisplayName` _favouriteplayerstart))
  (return _favouriteplayerstart))

(fn `UserConstructionScript`)