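; Survival player controller that creates and manages the player's UI: HUD, death screen, pause menu, hold-to-show map, inventory, loot menu and notifications.
; BeginPlay adds the main HUD in game-only input, while ShowIngameUI clears all widgets and rebuilds HUD and notification stack for the local controller.
; Most screens are recreated on each open, but inventory and notifications reuse their widgets.
; Loot and inventory block movement, with inventory also switching to UI-only mouse input.
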(event `self.ShowDeathScreen`
  (params (Killer :type "SurvivalCharacter Object Reference"))
  (bind _deathscreenwidget (`self.DeathScreenWidget`))
  ;[1 1 1] UI
  ;;[0 0 0] Death
  (`/Engine/EditorBlueprintResources/StandardMacros.IsValid` _deathscreenwidget
    (:`Is Valid`
      (`Widget.RemoveFromParent` _deathscreenwidget))
    (:`Is Not Valid`
      _))
  (bind _returnvalue (`|CreateWidget` "/Game/UserInterface/Widgets/Main/WBP_DeathScreen.WBP_DeathScreen_C" null Killer))
  (bind _output_get (set `self.DeathScreenWidget` _returnvalue))
  (`UserWidget.AddToViewport` _output_get 0)
  (bind _ingamewidget (`self.IngameWidget`)
    (:`then`
      (`Widget.RemoveFromParent` _ingamewidget))
    (:`else`)))

(event `InputAction|OpenPauseMenu`
  (params (Key :type "Key Structure"))
  (bind _pausemenuwidget (`self.PauseMenuWidget`))
  ;[1 1 1] UI
  ;;[0.05203 1 0.9901] InGame UI
  (:`Pressed`
    (`/Engine/EditorBlueprintResources/StandardMacros.IsValid` _pausemenuwidget
      (:`Is Valid`
        (`Widget.RemoveFromParent` _pausemenuwidget))
      (:`Is Not Valid`
        _))
    (bind _returnvalue (`|CreateWidget` "/Game/UserInterface/Widgets/MainMenu/WBP_PauseMenu.WBP_PauseMenu_C"))
    (bind _output_get (set `self.PauseMenuWidget` _returnvalue))
    (`UserWidget.AddToViewport` _output_get 0)))

(event `InputAction|OpenMap`
  (params (Key :type "Key Structure"))
  (bind _mapwidget (`self.MapWidget`))
  ;[1 1 1] UI
  ;;[0.05203 1 0.9901] InGame UI
  (:`Pressed`
    (`/Engine/EditorBlueprintResources/StandardMacros.IsValid` (`self.MapWidget`)
      (:`Is Valid`
        (`Widget.RemoveFromParent` _mapwidget))
      (:`Is Not Valid`
        _))
    (bind _returnvalue (`|CreateWidget` "/Game/UserInterface/Widgets/Main/WBP_Map.WBP_Map_C"))
    (bind _output_get (set `self.MapWidget` _returnvalue))
    (`UserWidget.AddToViewport` _output_get 0))
  (:`Released`
    (`/Engine/EditorBlueprintResources/StandardMacros.IsValid` (`self.MapWidget`)
      (:`Is Valid`
        (`Widget.RemoveFromParent` _mapwidget)))))

(event `self.OnHitPlayer`
  (bind _ingamewidget (`self.IngameWidget`))
  ;[1 1 1] UI
  ;;[0.05203 1 0.9901] InGame UI
  (`UserWidget.PlayAnimation` _ingamewidget (`/Game/UserInterface/Widgets/Main/WBP_Main.HitMarker_Anim` _ingamewidget) 0.0 1 "Forward" 1.0))

(event `self.ShowLootMenu`
  (params (LootSource :type "InventoryComponent Object Reference"))
  ;[1 1 1] UI
  ;;[0.025 0.1346 1] LootMenu
  (bind _returnvalue (`|CreateWidget` "/Game/UserInterface/Widgets/Inventory/WBP_LootMenu.WBP_LootMenu_C"))
  (bind _output_get (set `self.LootMenuWidget` _returnvalue))
  (`UserWidget.AddToViewport` _output_get 0)
  (`self.SetIgnoreMoveInput` true))

(event `self.HideLootMenu`
  ;[1 1 1] UI
  ;;[0.025 0.1346 1] LootMenu
  (`Widget.RemoveFromParent` (`self.LootMenuWidget`)))

(event `self.ShowNotificationMessage`
  (params (Message :type "Text (by ref)"))
  (bind _notificationwidget (`self.NotificationWidget`))
  ;[1 1 1] UI
  ;;[1 0 0.3049] Notifications
  (if (`self.IsLocalController`)
    (`/Engine/EditorBlueprintResources/StandardMacros.IsValid` _notificationwidget
      (:`Is Valid`
        (`/Game/UserInterface/Widgets/Main/WBP_NotificationStack.AddNotification` _notificationwidget Message)))))

(event `CreateNotificatioUI`
  ;[1 1 1] UI
  ;;[1 0 0.3049] Notifications
  (`/Engine/EditorBlueprintResources/StandardMacros.IsValid` (`self.NotificationWidget`)
    (:`Is Valid`
      _)
    (:`Is Not Valid`
      (bind _returnvalue (`|CreateWidget` "/Game/UserInterface/Widgets/Main/WBP_NotificationStack.WBP_NotificationStack_C" self))
      (set `self.NotificationWidget` _returnvalue)))
  (`UserWidget.AddToViewport` (`self.NotificationWidget`) 0))

(event `self.ShowIngameUI`
  ;[1 1 1] UI
  ;;[0 1 0.1767] BaseUI Actions
  (if (`self.IsLocalPlayerController`)
    (`WidgetLayoutLibrary.RemoveAllWidgets`)
    (`self.AddIngameUI`)
    (`self.CreateNotificatioUI`)))

(event `AddIngameUI`
  ;[1 1 1] UI
  ;;[0 1 0.1767] BaseUI Actions
  (`self.AddDefaultIngameUI`))

(event `InputAction|OpenInventory`
  (params (Key :type "Key Structure"))
  ;[1 1 1] Inventory
  (:`Pressed`
    (`|ExecutionSequence`
      (:`then_0`
        (`self.SetIgnoreMoveInput` true))
      (:`then_1`
        (if (not (`KismetSystemLibrary.IsValid` (`self.InventoryWidget`)))
          (bind _returnvalue (`|CreateWidget` (`self.InventoryClass`)))
          (set `self.InventoryWidget` _returnvalue))
        (`UserWidget.AddToViewport` (`self.InventoryWidget`) 0)
        (set `self.bShowMouseCursor` true)
        (`WidgetBlueprintLibrary.SetInputMode_UIOnlyEx` self (`self.InventoryWidget`))))))

(event `self.ReceiveBeginPlay`
  (`self.AddIngameUI`)
  (`WidgetBlueprintLibrary.SetInputMode_GameOnly` self)
  (set `self.bShowMouseCursor` false))

(fn `AddDefaultIngameUI`
  (bind _ingamewidget (`self.IngameWidget`))
  (bind _deathscreenwidget (`self.DeathScreenWidget`))
  (`/Engine/EditorBlueprintResources/StandardMacros.IsValid` _deathscreenwidget
    (:`Is Valid`
      (`Widget.RemoveFromParent` _deathscreenwidget))
    (:`Is Not Valid`
      _))
  (`/Engine/EditorBlueprintResources/StandardMacros.IsValid` _ingamewidget
    (:`Is Valid`
      (`Widget.RemoveFromParent` _ingamewidget))
    (:`Is Not Valid`
      _))
  (bind _returnvalue (`|CreateWidget` "/Game/UserInterface/Widgets/Main/WBP_Main.WBP_Main_C" self))
  (`/Engine/EditorBlueprintResources/StandardMacros.IsValid` _returnvalue
    (:`Is Valid`
      (set `self.IngameWidget` _returnvalue)
      (`UserWidget.AddToViewport` (`self.IngameWidget`) 0))))

(fn `UserConstructionScript`)